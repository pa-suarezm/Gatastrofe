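; BP_gato is a player-controlled character, named as a cat, that can move, look around and jump.
; Horizontal and vertical movement axes add movement input along the right and forward vectors of its StaticMesh component, so direction follows that mesh's orientation.
; Camera axes feed controller yaw and pitch, and the jump action starts jumping on press and stops on release.
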(event `InputAxis|movement_horizontal`
  (params (AxisValue :type "Float (single-precision)"))
  (`self.AddMovementInput` (`SceneComponent.GetRightVector` (`self.StaticMesh`)) AxisValue))

(event `InputAxis|movement_vertical`
  (params (AxisValue :type "Float (single-precision)"))
  (`self.AddMovementInput` (`SceneComponent.GetForwardVector` (`self.StaticMesh`)) AxisValue))

(event `InputAxis|camera_horizontal`
  (params (AxisValue :type "Float (single-precision)"))
  (`self.AddControllerYawInput` AxisValue))

(event `InputAxis|camera_vertical`
  (params (AxisValue :type "Float (single-precision)"))
  (`self.AddControllerPitchInput` AxisValue))

(event `InputAction|action_jump`
  (params (Key :type "Key Structure"))
  (:`Pressed`
    (`self.Jump`))
  (:`Released`
    (`self.StopJumping`)))

(fn `UserConstructionScript`)